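; Moving platform Blueprint that shuttles its Plateforme component back and forth between two points in the level.
; At BeginPlay it stores the locations of the first actors tagged "A" and "B", then starts Deplacements.
; A FlipFlop alternately plays and reverses a Timeline that lerps the world location without sweep, and the Timeline's Finished output re-calls Deplacements to loop the motion.
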(event Custom|Deplacements
  (Utilities|FlowControl|FlipFlop
    (:A
      (bind _newtrack_0 (Timeline|Timeline_0 PlayFromStart)
        (:Update
          (Transformation|SetWorldLocation (Variables|Default|GetPlateforme) (Math|Vector|Lerp(Vector) (Variables|Default|GetLocation%20A) (Variables|Default|GetLocation%20B) _newtrack_0) false false))
        (:Finished
          (CallFunction|Deplacements))))
    (:B
      (Timeline|Timeline_0 ReverseFromEnd))))

(event EventBeginPlay
  (Utilities|FlowControl|Sequence
    (:then_0
      (bind _outactors (Actor|GetAllActorswithTag "A"))
      (Variables|Default|SetLocation%20A (Transformation|GetActorLocation (Utilities|Array|Get(acopy) _outactors)))
      (bind _outactors_2 (Actor|GetAllActorswithTag "B"))
      (Variables|Default|SetLocation%20B (Transformation|GetActorLocation (Utilities|Array|Get(acopy) _outactors_2))))
    (:then_1
      (CallFunction|Deplacements))))

(fn ConstructionScript)