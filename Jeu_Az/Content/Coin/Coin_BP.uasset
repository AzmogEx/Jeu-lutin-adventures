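; Collectible coin pickup that spins and bobs, adding to the hero's coin count when collected.
; Tick rotates the mesh, while a FlipFlop alternately plays and reverses a timeline that offsets its height from the starting Z, re-triggering itself on finish.
; Overlapping the box with a Hero_BP plays a sound, increments that hero's Coin variable and destroys the actor.
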(event OnComponentBeginOverlap(Box)
  (params (OverlappedComponent :type Primitive%20Component%20Object%20Reference) (OtherActor :type Actor%20Object%20Reference) (OtherComp :type Primitive%20Component%20Object%20Reference) (OtherBodyIndex :type Integer) (bFromSweep :type Boolean) (SweepResult :type Hit%20Result%20Structure%20%28by%20ref%29))
  (bind _ashero_bp (Utilities|Casting|CastToHero_BP OtherActor))
  (Audio|SpawnSoundatLocation "/Game/Coin/CoinSoundEffect.CoinSoundEffect" (Transformation|GetActorLocation) "0, 0, 0" 0.5)
  (Math|Integer|IncrementInt (Variables|/Game/Hero/Hero_BP.Hero_BP_C|GetCoin _ashero_bp)
    (:%20%20
      (Actor|DestroyActor))))

(event Custom|Up/Down
  (bind _coinstaticmesh (Variables|Default|GetCoinStaticMesh))
  (bind _returnvalue (Transformation|GetWorldLocation _coinstaticmesh))
  (Utilities|FlowControl|FlipFlop
    (:A
      (bind _newtrack_1 (Timeline|Timeline_0 PlayFromStart)
        (:Update
          (Transformation|SetWorldLocation _coinstaticmesh (Math|Vector|MakeVector (.x _returnvalue) (.y _returnvalue) (+ (* _newtrack_1 1e+01) (Variables|Default|GetPositionZinitial))) false false))
        (:Finished
          (CallFunction|Up/Down))))
    (:B
      (Timeline|Timeline_0 ReverseFromEnd))))

(event EventBeginPlay
  (Variables|Default|SetPositionZinitial (.z (Transformation|GetWorldLocation (Variables|Default|GetCoinStaticMesh))))
  (CallFunction|Up/Down))

(event EventTick
  (params (DeltaSeconds :type Float%20%28single-precision%29))
  (Transformation|AddRelativeRotation (Variables|Default|GetCoinStaticMesh) "0,0.500000, 0" false false))

(fn ConstructionScript)